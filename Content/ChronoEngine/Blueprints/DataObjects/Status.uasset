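; Status data object in ChronoEngine that holds turn-based removal rules, made up of a removal type and an integer duration range.
; Its ValidatePropertyInformation event rebuilds those rules, clamping both duration bounds to zero or above while keeping the removal type and each bound's type intact.
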(event `self.ValidatePropertyInformation`
  (bind (_removaltype _durration) (break `/Game/ChronoEngine/Blueprints/DataObjects/VariableTypes/TurnRemovalRules` (`self.TurnRemovalRules`)))
  (bind (_lowerbound _upperbound) (break `Int32Range` _durration))
  (bind (_type _value) (break `Int32RangeBound` _lowerbound))
  (bind (_type_2 _value_2) (break `Int32RangeBound` _upperbound))
  (set `self.TurnRemovalRules` (make `/Game/ChronoEngine/Blueprints/DataObjects/VariableTypes/TurnRemovalRules` _removaltype (make `Int32Range` (make `Int32RangeBound` _type (`KismetMathLibrary.Max` _value)) (make `Int32RangeBound` _type_2 (`KismetMathLibrary.Max` _value_2))))))