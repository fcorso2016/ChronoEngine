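; SystemData is a ChronoEngine data object holding game-wide setup such as the starting party and map connection data.
; On property validation, ValidateParty removes repeated StartingParty entries by tracking those already seen in PartyMembers, removing by index during the forward loop.
; GetMapLocation looks up a map name in MapConnectionData, falling back to the name itself converted to a Name when no entry exists.
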(event `self.ValidatePropertyInformation`
  (`self.ValidateParty`))

(fn `GetMapLocation`
  (params (MapName :type String))
  (returns (LevelName :type Name))
  (bind (_value _returnvalue) (`BlueprintMapLibrary.Map_Find` (`self.MapConnectionData`) MapName))
  (if _returnvalue
    (return _value)
    (else
      (return (`KismetStringLibrary.Conv_StringToName` (`local.MapName`))))))

(fn `ValidateParty`
  (locals (PartyMembers :type "Set of /Game/RPGBasics/Blueprints/DataContainers/UnitData Object Reference"))
  (bind _startingparty (`self.StartingParty`))
  (for (_array_element _array_index) _startingparty
    (if (`BlueprintSetLibrary.Set_Contains` (`local.PartyMembers`) _array_element)
      (`KismetArrayLibrary.Array_Remove` _startingparty _array_index)
      (else
        (`BlueprintSetLibrary.Set_Add` (`local.PartyMembers`) _array_element)))))