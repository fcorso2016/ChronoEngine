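; HeroData is a data object for a hero that holds the hero's initial equipment.
; On property validation it checks each initial equipment slot, comparing the slot's equipment type with the class of the assigned piece.
; Slots that fail the check are replaced through DequipItem, which builds a slot that keeps only the equipment type.
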(event `self.ValidatePropertyInformation`
  (`self.ValidateEquipment`))