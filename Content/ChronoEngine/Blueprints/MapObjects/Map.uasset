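; Map actor that defines a playfield's edges and stops the top-down player's camera scrolling near them.
; The construction script sizes and positions four edge boxes from the map dimensions, and four camera-bound boxes that also factor in screen size.
; When the player's CharacterCenter box overlaps a camera bound, the camera boom's world X or Y is captured.
; Tick holds the boom at that coordinate until the overlap ends, leaving other axes free.
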(event `self.ReceiveTick`
  (params (DeltaSeconds :type "Float (single-precision)"))
  (bind _cameratolock (`self.CameraToLock`))
  (bind (_x _y) (`KismetMathLibrary.BreakVector2D` (`self.CameraPosition`)))
  (`parent.ReceiveTick` DeltaSeconds)
  (`/Engine/EditorBlueprintResources/StandardMacros.IsValid` (`self.CameraToLock`)
    (:`Is Valid`
      (`SceneComponent.K2_SetWorldLocation` _cameratolock (`KismetMathLibrary.MakeVector` (select `bool` (`self.LockX?`) :`false` (.x (`SceneComponent.K2_GetComponentLocation` _cameratolock)) :`true` _x) (select `bool` (`self.LockY?`) :`false` (.y (`SceneComponent.K2_GetComponentLocation` _cameratolock)) :`true` _y) (.z (`SceneComponent.K2_GetComponentLocation` _cameratolock))) false false))))

(event `self.TopCameraBounds.OnComponentBeginOverlap`
  (params (OverlappedComponent :type "PrimitiveComponent Object Reference") (OtherActor :type "Actor Object Reference") (OtherComp :type "PrimitiveComponent Object Reference") (OtherBodyIndex :type Integer) (bFromSweep :type Boolean) (SweepResult :type "HitResult Structure (by ref)"))
  (bind _playercharacter (`self.ValidateCollidedActor` OtherActor OtherComp))
  (`self.LockY` _playercharacter))

(event `self.TopCameraBounds.OnComponentEndOverlap`
  (params (OverlappedComponent :type "PrimitiveComponent Object Reference") (OtherActor :type "Actor Object Reference") (OtherComp :type "PrimitiveComponent Object Reference") (OtherBodyIndex :type Integer))
  (`self.ValidateCollidedActor` OtherActor OtherComp)
  (set `self.LockY?` false))

(event `self.BottomCameraBounds.OnComponentBeginOverlap`
  (params (OverlappedComponent :type "PrimitiveComponent Object Reference") (OtherActor :type "Actor Object Reference") (OtherComp :type "PrimitiveComponent Object Reference") (OtherBodyIndex :type Integer) (bFromSweep :type Boolean) (SweepResult :type "HitResult Structure (by ref)"))
  (bind _playercharacter (`self.ValidateCollidedActor` OtherActor OtherComp))
  (`self.LockY` _playercharacter))

(event `self.BottomCameraBounds.OnComponentEndOverlap`
  (params (OverlappedComponent :type "PrimitiveComponent Object Reference") (OtherActor :type "Actor Object Reference") (OtherComp :type "PrimitiveComponent Object Reference") (OtherBodyIndex :type Integer))
  (`self.ValidateCollidedActor` OtherActor OtherComp)
  (set `self.LockY?` false))

(event `self.LeftCameraBounds.OnComponentBeginOverlap`
  (params (OverlappedComponent :type "PrimitiveComponent Object Reference") (OtherActor :type "Actor Object Reference") (OtherComp :type "PrimitiveComponent Object Reference") (OtherBodyIndex :type Integer) (bFromSweep :type Boolean) (SweepResult :type "HitResult Structure (by ref)"))
  (bind _playercharacter (`self.ValidateCollidedActor` OtherActor OtherComp))
  (`self.LockX` _playercharacter))

(event `self.LeftCameraBounds.OnComponentEndOverlap`
  (params (OverlappedComponent :type "PrimitiveComponent Object Reference") (OtherActor :type "Actor Object Reference") (OtherComp :type "PrimitiveComponent Object Reference") (OtherBodyIndex :type Integer))
  (`self.ValidateCollidedActor` OtherActor OtherComp)
  (set `self.LockX?` false))

(event `self.RightCameraBounds.OnComponentBeginOverlap`
  (params (OverlappedComponent :type "PrimitiveComponent Object Reference") (OtherActor :type "Actor Object Reference") (OtherComp :type "PrimitiveComponent Object Reference") (OtherBodyIndex :type Integer) (bFromSweep :type Boolean) (SweepResult :type "HitResult Structure (by ref)"))
  (bind _playercharacter (`self.ValidateCollidedActor` OtherActor OtherComp))
  (`self.LockX` _playercharacter))

(event `self.RightCameraBounds.OnComponentEndOverlap`
  (params (OverlappedComponent :type "PrimitiveComponent Object Reference") (OtherActor :type "Actor Object Reference") (OtherComp :type "PrimitiveComponent Object Reference") (OtherBodyIndex :type Integer))
  (`self.ValidateCollidedActor` OtherActor OtherComp)
  (set `self.LockX?` false))

(fn `UserConstructionScript`
  (`self.PositionMapBounds`)
  (`self.PositionCameraBounds`))