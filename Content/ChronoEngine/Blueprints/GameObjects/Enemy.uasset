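; Enemy is a battle unit object in ChronoEngine whose name and stats come from an EnemyData object.
; Setup stores the game instance, owning side and data object, and GetEnemyData casts that stored UnitData to EnemyData.
; GetName appends an optional suffix to the data's name.
; GetBaseStat selects the requested stat from the data, returning zero when the data is invalid.
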(fn `GetBaseStat`
  (params (Stat :type "/Game/ChronoEngine/Blueprints/GameObjects/Stat Enum" :default "NewEnumerator0"))
  (returns (Value :type Integer))
  (bind _enemydata (`self.GetEnemyData`))
  (return (select `bool` (`KismetSystemLibrary.IsValid` _enemydata) :`true` (select `/Game/ChronoEngine/Blueprints/GameObjects/Stat` Stat :`NewEnumerator0` (`/Game/ChronoEngine/Blueprints/DataObjects/EnemyData.HP` _enemydata) :`NewEnumerator1` (`/Game/ChronoEngine/Blueprints/DataObjects/EnemyData.MP` _enemydata) :`NewEnumerator2` (`/Game/ChronoEngine/Blueprints/DataObjects/EnemyData.Attack` _enemydata) :`NewEnumerator3` (`/Game/ChronoEngine/Blueprints/DataObjects/EnemyData.Defense` _enemydata) :`NewEnumerator4` (`/Game/ChronoEngine/Blueprints/DataObjects/EnemyData.Magic` _enemydata) :`NewEnumerator5` (`/Game/ChronoEngine/Blueprints/DataObjects/EnemyData.Resistance` _enemydata) :`NewEnumerator6` (`/Game/ChronoEngine/Blueprints/DataObjects/EnemyData.Speed` _enemydata)))))

(fn `GetEnemyData`
  (returns (EnemyData :type "/Game/ChronoEngine/Blueprints/DataObjects/EnemyData Object Reference"))
  (bind _asenemy_data (cast `/Game/ChronoEngine/Blueprints/DataObjects/EnemyData` (`self.UnitData`))
    (:`then`
      (return _asenemy_data))
    (:`CastFailed`
      (return null))))

(fn `GetName`
  (returns (GetName :type Text))
  (bind _suffix (`self.Suffix`))
  (bind _name (`RPG_DataBase.Name` (`self.GetEnemyData`)))
  (return (select `bool` (`KismetTextLibrary.TextIsEmpty` _suffix) :`false` (`|FormatText` "{name} {suffix}" _name _suffix) :`true` _name)))

(fn `Setup`
  (params (GameInstance :type "GameInstance Object Reference") (OwningSide :type "/Game/RPGBasics/Blueprints/GameObjects/Side Object Reference") (DataObject :type "/Game/ChronoEngine/Blueprints/DataObjects/EnemyData Object Reference"))
  (`self.SetGameInstance` GameInstance)
  (set `self.OwningSide` OwningSide)
  (set `self.UnitData` DataObject))