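; AI_Faction is the object for an AI-controlled side, building and holding its enemy members from faction data.
; Setup stores the game instance, then creates an Enemy for each entry in the faction's enemy list and adds it to Members.
; Each Enemy is constructed with the faction as Outer and initialized with its data, the game instance and the faction as owning side.
; GetMembers exposes the resulting list.
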(fn `GetMembers`
  (returns (Members :type "Array of /Game/RPGBasics/Blueprints/GameObjects/Unit Object Reference"))
  (return (`self.Members`)))

(fn `Setup`
  (params (GameInstance :type "GameInstance Object Reference") (EnemyFaction :type "/Game/ChronoEngine/Blueprints/Combat/EnemyFaction Structure"))
  (`self.SetGameInstance` GameInstance)
  (for _array_element (`.Enemies_13_586CCAC94946BCD49D5FB4A7BE28664A` (break `/Game/ChronoEngine/Blueprints/Combat/EnemyFaction` EnemyFaction))
    (bind _constructedenemy (`self.CreateEnemy` (`.EnemyData_2_FE98DC474AFE8738F18B3AAFB35C4823` (break `/Game/ChronoEngine/Blueprints/Combat/EnemyPawnPair` _array_element))))
    (`KismetArrayLibrary.Array_Add` (`self.Members`) _constructedenemy)))