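; Party object that tracks the player's hero roster and whether it is in battle.
; Setup stores the game instance and fills the roster from the StartingParty system setting.
; GetMembers resolves roster entries to heroes through ChronoGameInstance, returning all outside battle and a leading subset during battle.
; That subset's size check runs after each add, so it can hold one more than the party maximum.
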(fn `GetActiveMembers`
  (returns (Members :type "Array of /Game/ChronoEngine/Blueprints/GameObjects/Hero Object Reference"))
  (locals (MemberList :type "Array of /Game/ChronoEngine/Blueprints/GameObjects/Hero Object Reference"))
  (for (_array_element _array_index) (`self.Members`)
    (`self.AddHeroToList` _array_element (`local.MemberList`))
    (if (>= _array_index (`self.GetMaxPartyMembers`))
      (break)))
  (return (`local.MemberList`)))

(fn `GetAllMembers`
  (returns (Members :type "Array of /Game/ChronoEngine/Blueprints/GameObjects/Hero Object Reference"))
  (locals (MemberList :type "Array of /Game/ChronoEngine/Blueprints/GameObjects/Hero Object Reference"))
  (for _array_element (`self.Members`)
    (`self.AddHeroToList` _array_element (`local.MemberList`)))
  (return (`local.MemberList`)))

(fn `GetMaxPartyMembers`
  (returns (MemberCount :type Integer))
  (return 3))

(fn `GetMembers`
  (returns (Members :type "Array of /Game/RPGBasics/Blueprints/GameObjects/Unit Object Reference"))
  (return (select `bool` (`self.InBattle?`) :`false` (`self.GetAllMembers`) :`true` (`self.GetActiveMembers`))))

(fn `InBattle?`
  (returns (InBattle :type Boolean))
  (return (`self.InBattle`)))

(fn `InitializeMembers`
  (bind _aschrono_game_instance (`self.RetrieveGameInstance`))
  (bind _output_get (set `self.Members` (`/Game/ChronoEngine/Blueprints/DataObjects/SystemData.StartingParty` (`/Game/ChronoEngine/Blueprints/System/ChronoGameInstance.SystemSettings` _aschrono_game_instance))))
  (`KismetArrayLibrary.Array_RemoveItem` _output_get))

(fn `OnBattleEnd`
  (set `self.InBattle` false))

(fn `OnStartBattle`
  (set `self.InBattle` true))

(fn `Setup`
  (params (GameInstance :type "GameInstance Object Reference"))
  (`self.SetGameInstance` GameInstance)
  (`self.InitializeMembers`))