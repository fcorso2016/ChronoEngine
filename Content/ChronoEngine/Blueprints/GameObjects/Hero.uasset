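; Hero is the player-controlled unit object, holding name, level, skills, HP, MP and status effects on top of inherited unit data.
; Setup initializes it from a data asset, and base stats come from HeroData curve tables evaluated at the clamped level, except Speed, which is flat.
; In battle, SelectAction hands action choice to the BattleHUD.
; SaveHero and LoadHero convert its state to and from a save struct.
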(event `self.SelectAction`
  (params (OnInputComplete :type "Delegate (by ref)") (Object :type "Object Object Reference"))
  (bind _asbattle (cast `/Game/RPGBasics/Blueprints/Combat/Battle` Object))
  (bind _asbattle_hud (cast `/Game/ChronoEngine/UI/Combat/Menus/BattleHUD` (`/Game/RPGBasics/Blueprints/Combat/Battle.HUD` _asbattle)))
  (`ActionSelector.SelectAction` _asbattle_hud OnInputComplete self))

(fn `EvaluateStatCurve`
  (params (Curve :type "CurveTableRowHandle Structure"))
  (returns (Stat :type Integer))
  (bind (_curvetable _rowname) (break `CurveTableRowHandle` Curve))
  (bind _outxy (`DataTableFunctionLibrary.EvaluateCurveTableRow` _curvetable _rowname (`KismetMathLibrary.Conv_IntToDouble` (`self.GetLevel`)) "StatCurve")
    (:`RowFound`
      (return (`KismetMathLibrary.FTrunc` _outxy)))
    (:`RowNotFound`
      (return 0))))

(fn `GetBaseStat`
  (params (Stat :type "/Game/ChronoEngine/Blueprints/GameObjects/Stat Enum" :default "NewEnumerator0"))
  (returns (Value :type Integer))
  (bind _herodata (`self.GetHeroData`))
  (return (select `bool` (`KismetSystemLibrary.IsValid` _herodata) :`true` (select `/Game/ChronoEngine/Blueprints/GameObjects/Stat` Stat :`NewEnumerator0` (`self.EvaluateStatCurve` (`/Game/ChronoEngine/Blueprints/DataObjects/HeroData.BaseHP` _herodata)) :`NewEnumerator1` (`self.EvaluateStatCurve` (`/Game/ChronoEngine/Blueprints/DataObjects/HeroData.BaseMP` _herodata)) :`NewEnumerator2` (`self.EvaluateStatCurve` (`/Game/ChronoEngine/Blueprints/DataObjects/HeroData.BaseAttack` _herodata)) :`NewEnumerator3` (`self.EvaluateStatCurve` (`/Game/ChronoEngine/Blueprints/DataObjects/HeroData.BaseDefense` _herodata)) :`NewEnumerator4` (`self.EvaluateStatCurve` (`/Game/ChronoEngine/Blueprints/DataObjects/HeroData.BaseMagic` _herodata)) :`NewEnumerator5` (`self.EvaluateStatCurve` (`/Game/ChronoEngine/Blueprints/DataObjects/HeroData.BaseResistance` _herodata)) :`NewEnumerator6` (`/Game/ChronoEngine/Blueprints/DataObjects/HeroData.BaseSpeed` _herodata)))))

(fn `GetHeroData`
  (returns (HeroData :type "/Game/ChronoEngine/Blueprints/DataObjects/HeroData Object Reference"))
  (bind _ashero_data (cast `/Game/ChronoEngine/Blueprints/DataObjects/HeroData` (`self.UnitData`))
    (:`then`
      (return _ashero_data))
    (:`CastFailed`
      (return null))))

(fn `GetLevel`
  (returns (Level :type Integer))
  (return (`self.Level`)))

(fn `GetMaxLevel`
  (returns (MaxLevel :type Integer))
  (bind _herodata (`self.GetHeroData`))
  (return (select `bool` (`KismetSystemLibrary.IsValid` _herodata) :`false` 99 :`true` (`/Game/ChronoEngine/Blueprints/DataObjects/HeroData.MaxLevel` _herodata))))

(fn `GetName`
  (returns (GetName :type Text))
  (return (`self.Name`)))

(fn `LoadHero`
  (params (Save :type "/Game/ChronoEngine/Blueprints/Saving/HeroSave Structure (by ref)"))
  (bind (_name _level _hp _mp _skills _statuseffects) (break `/Game/ChronoEngine/Blueprints/Saving/HeroSave` Save))
  (set `self.Name` _name)
  (`self.SetLevel` _level)
  (`self.SetCurrentHP` _hp)
  (`self.SetCurrentMP` _mp)
  (set `self.Skills` _skills)
  (set `self.StatusEffects` _statuseffects)
  (return))

(fn `SaveHero`
  (returns (Save :type "/Game/ChronoEngine/Blueprints/Saving/HeroSave Structure"))
  (return (make `/Game/ChronoEngine/Blueprints/Saving/HeroSave` (`self.Name`) (`self.Level`) (`self.HP`) (`self.MP`) (`self.Skills`) (`self.StatusEffects`))))

(fn `SetLevel`
  (params (Level :type Integer))
  (set `self.Level` (`KismetMathLibrary.Clamp` Level 1 (`self.GetMaxLevel`))))

(fn `Setup`
  (params (GameInstance :type "GameInstance Object Reference") (OwningSide :type "/Game/RPGBasics/Blueprints/GameObjects/Side Object Reference") (DataObject :type "/Game/ChronoEngine/Blueprints/DataObjects/HeroData Object Reference"))
  (`self.SetGameInstance` GameInstance)
  (set `self.OwningSide` OwningSide)
  (set `self.UnitData` DataObject)
  (set `self.Level` (`/Game/ChronoEngine/Blueprints/DataObjects/HeroData.StartingLevel` DataObject))
  (set `self.Name` (`RPG_DataBase.Name` DataObject))
  (set `self.Skills` (`/Game/ChronoEngine/Blueprints/DataObjects/HeroData.StartingSkills` DataObject))
  (`self.SetCurrentHP` (`self.GetMaxHP`))
  (`self.SetCurrentMP` (`self.GetMaxMP`)))