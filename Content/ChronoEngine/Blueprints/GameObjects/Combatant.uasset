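; Base combatant for ATB battles, providing stats, MP, skill cost checks and a speed-driven gauge that fires an event when full.
; Stats combine placeholder base and bonus getters, presumably for child overrides, with status-effect multipliers, then clamp.
; A status map stores turn counters and alters damage rates; effects expire on action, turn, battle-end or damage hooks, posting HUD messages.
; Death hides the linked world actor and disables collision; positive HP restores both.
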(event `self.Die`
  (`parent.Die`)
  (`self.SetAppearanceAsKnockedOut`))

(event `self.SetCurrentHP`
  (params (NewHP :type Integer))
  (`parent.SetCurrentHP` NewHP)
  (if (> NewHP 0)
    (`self.SetAppearanceAsOK`)))

(fn `AddMessageToHUD`
  (params (Line :type Text))
  (bind _owningbattle (`self.OwningBattle`))
  (`/Engine/EditorBlueprintResources/StandardMacros.IsValid` _owningbattle
    (:`Is Valid`
      (bind _asbattle_hud (cast `/Game/ChronoEngine/UI/Combat/Menus/BattleHUD` (`/Game/RPGBasics/Blueprints/Combat/Battle.HUD` _owningbattle)))
      (`/Game/ChronoEngine/UI/Combat/Menus/BattleHUD.AddBattleMessage` _asbattle_hud Line true))))

(fn `AddStatusEffect`
  (params (Status :type "/Game/ChronoEngine/Blueprints/DataObjects/Status Object Reference"))
  (`BlueprintMapLibrary.Map_Add` (`self.StatusEffects`) Status (select `bool` (!= (`KismetMathLibrary.And_IntInt` (`|BitmaskLiteral` 2) (`/Game/ChronoEngine/Blueprints/DataObjects/Status.RemovalType` Status)) 0) :`true` (`self.GetRandomTurnInRange` Status))))

(fn `ATB_Max`
  (returns (Max :type "Float (double-precision)"))
  (return 100.0))

(fn `ATB_Tick`
  (params (DeltaSeconds :type "Float (double-precision)"))
  (bind _atb_fill (`self.ATB_Fill`))
  (if (< _atb_fill (`self.ATB_Max`))
    (bind _output_get (set `self.ATB_Fill` (`KismetMathLibrary.FClamp` (+ (* DeltaSeconds (`KismetMathLibrary.Conv_IntToDouble` (`self.GetBattleSpeed`)) 5.0) _atb_fill) 0.0 (`self.ATB_Max`))))
    (if (>= _output_get (`self.ATB_Max`))
      (`self.OnATB_Full` self))))

(fn `CanUse?`
  (params (Action :type "/Game/RPGBasics/Blueprints/DataContainers/Action Object Reference"))
  (returns (`Usable?` :type Boolean))
  (bind _asskill (cast `/Game/ChronoEngine/Blueprints/DataObjects/Skill` Action)
    (:`then`
      (return (>= (`self.GetCurrentMP`) (`/Game/ChronoEngine/Blueprints/DataObjects/Skill.MP_Cost` _asskill))))
    (:`CastFailed`
      (return (`parent.CanUse?` Action)))))

(fn `FillATB`
  (bind _max (`self.ATB_Max`))
  (if (< (`self.ATB_Fill`) _max)
    (set `self.ATB_Fill` _max)
    (`self.OnATB_Full` self)))

(fn `GetAttack`
  (returns (Attack :type Integer))
  (return (`self.GetStat` "NewEnumerator2")))

(fn `GetBaseStat`
  (params (Stat :type "/Game/ChronoEngine/Blueprints/GameObjects/Stat Enum" :default "NewEnumerator0"))
  (returns (Value :type Integer))
  (return 0))

(fn `GetBattleSpeed`
  (returns (Speed :type Integer))
  (return (`self.GetSpeed`)))

(fn `GetCriticalChance`
  (returns (Critical :type Integer))
  (return 4))

(fn `GetCurrentMP`
  (returns (MP :type Integer))
  (return (`self.MP`)))

(fn `GetDamageRate`
  (params (AttckType :type "/Game/RPGBasics/Blueprints/Combat/Modules/BaseClasses/AttackType Enum" :default "NewEnumerator0"))
  (returns (DamageRate :type "Float (double-precision)"))
  (locals (Mult :type "Float (double-precision)" :default 0.0))
  (set `local.Mult` (`parent.GetDamageRate` AttckType))
  (bind _keys (`BlueprintMapLibrary.Map_Keys` (`self.StatusEffects`)))
  (for _array_element _keys
    (bind (_value _returnvalue) (`BlueprintMapLibrary.Map_Find` (`/Game/ChronoEngine/Blueprints/DataObjects/Status.DamageRates` _array_element) AttckType))
    (if _returnvalue
      (set `local.Mult` _value)))
  (return (`local.Mult`)))

(fn `GetDefense`
  (returns (Defense :type Integer))
  (return (`self.GetStat` "NewEnumerator3")))

(fn `GetEvasion`
  (returns (Evasion :type Integer))
  (return 5))

(fn `GetHit`
  (returns (Hit :type Integer))
  (return 95))

(fn `GetLevel`
  (returns (Level :type Integer))
  (return 0))

(fn `GetMagic`
  (returns (Magic :type Integer))
  (return (`self.GetStat` "NewEnumerator4")))

(fn `GetMaxHP`
  (returns (HP :type Integer))
  (return (`self.GetStat` "NewEnumerator0")))

(fn `GetMaxMP`
  (returns (MP :type Integer))
  (return (`self.GetStat` "NewEnumerator1")))

(fn `GetName`
  (returns (GetName :type Text))
  (return ""))

(fn `GetResistance`
  (returns (Resistance :type Integer))
  (return (`self.GetStat` "NewEnumerator5")))

(fn `GetSpeed`
  (returns (Speed :type Integer))
  (return (`self.GetStat` "NewEnumerator6")))

(fn `GetStat`
  (params (Stat :type "/Game/ChronoEngine/Blueprints/GameObjects/Stat Enum" :default "NewEnumerator0"))
  (returns (Value :type Integer))
  (return (`KismetMathLibrary.Clamp` (`KismetMathLibrary.FTrunc` (+ (* (`self.GetBaseStat` Stat) (`self.GetStatMultipliers` Stat)) (`KismetMathLibrary.Conv_IntToDouble` (`self.GetStatBonus` Stat)))) (`self.GetStatMin` "NewEnumerator0") (`self.GetStatMax` "NewEnumerator0"))))

(fn `GetStatBonus`
  (params (Stat :type "/Game/ChronoEngine/Blueprints/GameObjects/Stat Enum" :default "NewEnumerator0"))
  (returns (Bonus :type Integer))
  (return 0))

(fn `GetStatMax`
  (params (Stat :type "/Game/ChronoEngine/Blueprints/GameObjects/Stat Enum" :default "NewEnumerator0"))
  (returns (Max :type Integer))
  (return (select `bool` (`|EnumEquality` Stat "NewEnumerator6") :`false` 999 :`true` 16)))

(fn `GetStatMin`
  (params (Stat :type "/Game/ChronoEngine/Blueprints/GameObjects/Stat Enum" :default "NewEnumerator0"))
  (returns (Max :type Integer))
  (return (select `bool` (`|EnumEquality` Stat "NewEnumerator1") :`false` 1)))

(fn `GetStatMultipliers`
  (params (Stat :type "/Game/ChronoEngine/Blueprints/GameObjects/Stat Enum" :default "NewEnumerator0"))
  (returns (Multiplier :type "Float (double-precision)"))
  (locals (Mult :type "Float (double-precision)" :default 1.0))
  (bind _keys (`BlueprintMapLibrary.Map_Keys` (`self.StatusEffects`)))
  (for _array_element _keys
    (bind (_value _returnvalue) (`BlueprintMapLibrary.Map_Find` (`/Game/ChronoEngine/Blueprints/DataObjects/Status.StatRates` _array_element) Stat))
    (if _returnvalue
      (set `local.Mult` _value)))
  (return (`local.Mult`)))

(fn `HasStatusEffect?`
  (params (Status :type "/Game/ChronoEngine/Blueprints/DataObjects/Status Object Reference"))
  (returns (`HasStatus?` :type Boolean))
  (return (`BlueprintMapLibrary.Map_Contains` (`self.StatusEffects`) Status)))

(fn `OnActionEnd`
  (`parent.OnActionEnd`)
  (`self.ProcessAutoStatusRemoval` "NewEnumerator2"))

(fn `OnBattleEnd`
  (`parent.OnBattleEnd`)
  (bind _keys (`BlueprintMapLibrary.Map_Keys` (`self.StatusEffects`)))
  (for _array_element _keys
    (if (!= (`KismetMathLibrary.And_IntInt` (`/Game/ChronoEngine/Blueprints/DataObjects/Status.RemovalType` _array_element) (`|BitmaskLiteral` 1)) 0)
      (`self.AddMessageToHUD` (`/Game/ChronoEngine/Blueprints/DataObjects/Status.GenerateRemoveMessage` _array_element (`self.GetName`)))
      (`self.RemoveStatusEffect` _array_element))))

(fn `OnDamage`
  (params (Damage :type Integer))
  (`parent.OnDamage` Damage)
  (bind _keys (`BlueprintMapLibrary.Map_Keys` (`self.StatusEffects`)))
  (for _array_element _keys
    (if (and (!= (`KismetMathLibrary.And_IntInt` (`/Game/ChronoEngine/Blueprints/DataObjects/Status.RemovalType` _array_element) (`|BitmaskLiteral` 1)) 0) (>= Damage (`/Game/ChronoEngine/Blueprints/DataObjects/Status.DamageToRemove` _array_element)))
      (`self.AddMessageToHUD` (`/Game/ChronoEngine/Blueprints/DataObjects/Status.GenerateRemoveMessage` _array_element (`self.GetName`)))
      (`self.RemoveStatusEffect` _array_element))))

(fn `OnTurnEnd`
  (`parent.OnTurnEnd`)
  (`self.ProcessAutoStatusRemoval` "NewEnumerator1"))

(fn `Pay/RestoreMP`
  (params (MP_Change :type Integer) (ChangeType :type "/Game/RPGBasics/Blueprints/GameObjects/ChangeType Enum" :default "NewEnumerator0"))
  (switch `/Game/RPGBasics/Blueprints/GameObjects/ChangeType` ChangeType
    (:`NewEnumerator0`
      (`self.SetCurrentMP` (+ (`self.GetCurrentMP`) MP_Change)))
    (:`NewEnumerator1`
      (`self.SetCurrentMP` (- (`self.GetCurrentMP`) MP_Change)))))

(fn `ProcessAutoStatusRemoval`
  (params (RemovalType :type "/Game/ChronoEngine/Blueprints/DataObjects/VariableTypes/TurnRemovalType Enum" :default "NewEnumerator1"))
  (bind _keys (`BlueprintMapLibrary.Map_Keys` (`self.StatusEffects`)))
  (for _array_element _keys
    (bind (_value _returnvalue) (`BlueprintMapLibrary.Map_Find` (`self.StatusEffects`) _array_element))
    (if (and _returnvalue (!= (`KismetMathLibrary.And_IntInt` (`/Game/ChronoEngine/Blueprints/DataObjects/Status.RemovalType` _array_element) (`|BitmaskLiteral` 2)) 0) (`|EnumEquality` (`.RemovalType_3_30376F12439A0B78D15574AC76795410` (break `/Game/ChronoEngine/Blueprints/DataObjects/VariableTypes/TurnRemovalRules` (`/Game/ChronoEngine/Blueprints/DataObjects/Status.TurnRemovalRules` _array_element))) RemovalType))
      (bind _result (`/Engine/EditorBlueprintResources/StandardMacros.DecrementInt` _value)
        (:`  `
          (if (< _result 0)
            (`self.AddMessageToHUD` (`/Game/ChronoEngine/Blueprints/DataObjects/Status.GenerateRemoveMessage` _array_element (`self.GetName`)))
            (`self.RemoveStatusEffect` _array_element)))))))

(fn `RemoveStatusEffect`
  (params (Status :type "/Game/ChronoEngine/Blueprints/DataObjects/Status Object Reference"))
  (`BlueprintMapLibrary.Map_Remove` (`self.StatusEffects`) Status))

(fn `ResetATB`
  (set `self.ATB_Fill` 0.0))

(fn `SetAppearanceAsKnockedOut`
  (bind _worldrepresentation (`self.WorldRepresentation`))
  (`/Engine/EditorBlueprintResources/StandardMacros.IsValid` _worldrepresentation
    (:`Is Valid`
      (`Actor.SetActorHiddenInGame` _worldrepresentation true)
      (`Actor.SetActorEnableCollision` _worldrepresentation false))))

(fn `SetAppearanceAsOK`
  (bind _worldrepresentation (`self.WorldRepresentation`))
  (`/Engine/EditorBlueprintResources/StandardMacros.IsValid` _worldrepresentation
    (:`Is Valid`
      (`Actor.SetActorHiddenInGame` _worldrepresentation false)
      (`Actor.SetActorEnableCollision` _worldrepresentation true))))

(fn `SetCurrentMP`
  (params (MP :type Integer))
  (set `self.MP` (`KismetMathLibrary.Clamp` MP 0 (`self.GetMaxMP`))))

(fn `SetWorldRepresentation`
  (params (NewRepresentation :type "Actor Object Reference"))
  (set `self.WorldRepresentation` NewRepresentation))