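; ATB_Battle is a battle Blueprint that runs Active Time Battle combat, notifying the game instance's party when battle starts.
; Each Tick advances every participant's ATB while combat flows, which IsCombatFlowing currently always allows.
; Retrieving context adds the party as a side and binds each combatant's ATB-full callback to begin that character's action selection.
; It also creates and sets up the BattleHUD widget.
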(event `self.BattleStart`
  (bind _aschrono_game_instance (cast `/Game/ChronoEngine/Blueprints/System/ChronoGameInstance` (`GameplayStatics.GetGameInstance`)))
  (`/Game/ChronoEngine/Blueprints/GameObjects/Party.OnStartBattle` (`/Game/ChronoEngine/Blueprints/System/ChronoGameInstance.GetParty` _aschrono_game_instance))
  (`parent.BattleStart`))

(event `self.ReceiveTick`
  (params (DeltaSeconds :type "Float (single-precision)"))
  (if (`self.IsCombatFlowing?`)
    (for _array_element (`self.GetAllParticipants`)
      (bind _ascombatant (cast `/Game/ChronoEngine/Blueprints/GameObjects/Combatant` _array_element))
      (`/Game/ChronoEngine/Blueprints/GameObjects/Combatant.ATB_Tick` _ascombatant DeltaSeconds))))

(event `self.RetrieveContextInformation`
  (`self.AddSidesToBattle`)
  (for _array_element (`self.GetAllParticipants`)
    (bind _ascombatant (cast `/Game/ChronoEngine/Blueprints/GameObjects/Combatant` _array_element))
    (add `/Game/ChronoEngine/Blueprints/GameObjects/Combatant.OnATB_Full` _ascombatant (delegate `OnATB_Fill`))))

(event `OnATB_Fill`
  (params (Character :type "/Game/ChronoEngine/Blueprints/GameObjects/Combatant Object Reference"))
  (`self.BeginActionSelection` Character))

(fn `AddSidesToBattle`
  (bind _aschrono_game_instance (cast `/Game/ChronoEngine/Blueprints/System/ChronoGameInstance` (`GameplayStatics.GetGameInstance`)))
  (`KismetArrayLibrary.Array_Add` (`self.Sides`) (`/Game/ChronoEngine/Blueprints/System/ChronoGameInstance.GetParty` _aschrono_game_instance)))

(fn `CreateHUD`
  (returns (HUD :type "UserWidget Object Reference"))
  (bind _returnvalue (`|CreateWidget` "/Game/ChronoEngine/UI/Combat/Menus/BattleHUD.BattleHUD_C" (`GameplayStatics.GetPlayerController` 0)))
  (`/Game/ChronoEngine/UI/Combat/Menus/BattleHUD.Setup` _returnvalue)
  (return _returnvalue))

(fn `IsCombatFlowing?`
  (returns (`Flowing?` :type Boolean))
  (return true))

(fn `UserConstructionScript`
  (`parent.UserConstructionScript`))