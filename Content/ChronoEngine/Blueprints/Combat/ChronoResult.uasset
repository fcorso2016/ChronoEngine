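; ChronoResult is a combat result record that collects MP changes and status changes, and tracks an overall Success flag.
; ProcessMPChanges stores the latest MP change, while AddStatus and RemoveStatus append unique entries to their added and removed lists.
; Success latches on a nonzero MP change or newly added status.
; RemoveStatus inverts that index check, setting Success only when the status is already listed as removed.
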(fn `AddStatus`
  (params (Status :type "/Game/ChronoEngine/Blueprints/DataObjects/Status Object Reference"))
  (bind _returnvalue (`KismetArrayLibrary.Array_AddUnique` (`self.StatusesAdded`) Status))
  (set `self.Success?` (or (!= _returnvalue (`ChronoCodeUtilities.GetNullIndex`)) (`self.Success?`))))

(fn `ProcessMPChanges`
  (params (Change :type Integer))
  (bind _output_get (set `self.MP_Change` Change))
  (set `self.Success?` (or (!= _output_get 0) (`self.Success?`))))

(fn `RemoveStatus`
  (params (Status :type "/Game/ChronoEngine/Blueprints/DataObjects/Status Object Reference"))
  (bind _returnvalue (`KismetArrayLibrary.Array_AddUnique` (`self.StatusesRemoved`) Status))
  (set `self.Success?` (or (== _returnvalue (`ChronoCodeUtilities.GetNullIndex`)) (`self.Success?`))))