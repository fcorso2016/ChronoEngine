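; ChronoPlayerController is a player controller Blueprint that tells the ChronoCameraManager which pawn is the player character.
; On both possess and unpossess, it passes the valid pawn to SetPlayerCharacter, so unpossessing sets the released pawn rather than clearing it.
; GetCameraManager looks up the controller by its own ID and casts its PlayerCameraManager to ChronoCameraManager, with no validity check by callers.
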(event `self.ReceivePossess`
  (params (PossessedPawn :type "Pawn Object Reference"))
  (`/Engine/EditorBlueprintResources/StandardMacros.IsValid` PossessedPawn
    (:`Is Valid`
      (`ChronoCameraManager.SetPlayerCharacter` (`self.GetCameraManager`) PossessedPawn))))

(event `self.ReceiveUnPossess`
  (params (UnpossessedPawn :type "Pawn Object Reference"))
  (`/Engine/EditorBlueprintResources/StandardMacros.IsValid` UnpossessedPawn
    (:`Is Valid`
      (`ChronoCameraManager.SetPlayerCharacter` (`self.GetCameraManager`) UnpossessedPawn))))

(fn `GetCameraManager`
  (returns (CameraManager :type "ChronoCameraManager Object Reference"))
  (bind _aschrono_camera_manager (cast `ChronoCameraManager` (`PlayerController.PlayerCameraManager` (`GameplayStatics.GetPlayerController` (`GameplayStatics.GetPlayerControllerID` self))))
    (:`then`
      (return _aschrono_camera_manager))
    (:`CastFailed`
      (return null))))

(fn `UserConstructionScript`)