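; ChronoGameMode is the game mode that sets up the current map and player when play begins.
; It stream-loads the map named in ChronoGameInstance, falling back to a debug start map when none is set, with a blocking load.
; If the instance flags a saved location, it moves the player character there and clears the flag.
; It then calls InitializePlayer on every Map actor.
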(event `self.ReceiveBeginPlay`
  (bind _aschrono_game_instance (cast `/Game/ChronoEngine/Blueprints/System/ChronoGameInstance` (`GameplayStatics.GetGameInstance`)))
  (bind _currentmap (`/Game/ChronoEngine/Blueprints/System/ChronoGameInstance.CurrentMap` _aschrono_game_instance))
  (`GameplayStatics.LoadStreamLevel` (select `bool` (<= (`KismetStringLibrary.Len` _currentmap) 0) :`false` (`KismetStringLibrary.Conv_StringToName` _currentmap) :`true` (`self.GetDebugStartMap`)) true true)
  (if (`/Game/ChronoEngine/Blueprints/System/ChronoGameInstance.LoadSavedLocation?` _aschrono_game_instance)
    (`self.K2_SetActorLocation` (`GameplayStatics.GetPlayerCharacter` 0) (`/Game/ChronoEngine/Blueprints/System/ChronoGameInstance.StartingLocation` _aschrono_game_instance) false false)
    (set `/Game/ChronoEngine/Blueprints/System/ChronoGameInstance.LoadSavedLocation?` false _aschrono_game_instance))
  (bind _outactors (`GameplayStatics.GetAllActorsOfClass` "/Game/ChronoEngine/Blueprints/MapObjects/Map.Map_C"))
  (for _array_element _outactors
    (`/Game/ChronoEngine/Blueprints/MapObjects/Map.InitializePlayer` _array_element)))

(fn `UserConstructionScript`)