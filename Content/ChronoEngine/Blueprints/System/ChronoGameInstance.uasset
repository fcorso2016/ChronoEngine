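; ChronoGameInstance is the game instance that owns the player's Party and Hero objects.
; GetParty lazily constructs a single Party with the game instance as outer, runs its Setup and caches it.
; GetHero returns the Hero cached in a map keyed by HeroData, or constructs one, sets it up with the Party as its owning side and stores it.
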(fn `GetHero`
  (params (HeroData :type "/Game/ChronoEngine/Blueprints/DataObjects/HeroData Object Reference"))
  (returns (Hero :type "/Game/ChronoEngine/Blueprints/GameObjects/Hero Object Reference"))
  (locals (CreatedHero :type "/Game/ChronoEngine/Blueprints/GameObjects/Hero Object Reference"))
  (bind (_value _returnvalue) (`BlueprintMapLibrary.Map_Find` (`self.Heroes`) HeroData))
  (if _returnvalue
    (return _value)
    (else
      (bind _returnvalue_2 (`|GenericCreateObject` "/Game/ChronoEngine/Blueprints/GameObjects/Hero.Hero_C" self))
      (bind _output_get (set `local.CreatedHero` _returnvalue_2))
      (`/Game/ChronoEngine/Blueprints/GameObjects/Hero.Setup` _output_get self (`self.GetParty`) HeroData)
      (`BlueprintMapLibrary.Map_Add` (`self.Heroes`) HeroData (`local.CreatedHero`))
      (return _output_get))))

(fn `GetParty`
  (returns (Party :type "/Game/ChronoEngine/Blueprints/GameObjects/Party Object Reference"))
  (`/Engine/EditorBlueprintResources/StandardMacros.IsValid` (`self.Party`)
    (:`Is Valid`
      _)
    (:`Is Not Valid`
      (bind _returnvalue (`|GenericCreateObject` "/Game/ChronoEngine/Blueprints/GameObjects/Party.Party_C" self))
      (bind _output_get (set `self.Party` _returnvalue))
      (`/Game/ChronoEngine/Blueprints/GameObjects/Party.Setup` _output_get self)))
  (return _output_get))