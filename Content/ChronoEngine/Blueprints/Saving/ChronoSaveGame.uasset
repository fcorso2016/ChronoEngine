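; Save game object for ChronoEngine that snapshots and restores game progress held in the game instance.
; SaveGameInstance stores party and per-hero saves (keyed by hero data), the current map, player location, visited maps, opened chests and event flags, switches and typed variables.
; LoadGameInstance hands party and hero saves back to their owners, copies the world and event state back, then warps to the saved map and location.
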(fn `LoadGameInstance`
  (params (GameInstance :type "/Game/ChronoEngine/Blueprints/System/ChronoGameInstance Object Reference"))
  (`/Game/ChronoEngine/Blueprints/GameObjects/Party.LoadParty` (`/Game/ChronoEngine/Blueprints/System/ChronoGameInstance.GetParty` GameInstance) (`self.Party`))
  (bind _keys (`BlueprintMapLibrary.Map_Keys` (`self.Heros`)))
  (for _array_element _keys
    (`/Game/ChronoEngine/Blueprints/GameObjects/Hero.LoadHero` (`/Game/ChronoEngine/Blueprints/System/ChronoGameInstance.GetHero` GameInstance _array_element) (`BlueprintMapLibrary.Map_Find` (`self.Heros`) _array_element)))
  (set `/Game/ChronoEngine/Blueprints/System/ChronoGameInstance.VisitedMaps` (`self.VisitedMaps`) GameInstance)
  (set `/Game/ChronoEngine/Blueprints/System/ChronoGameInstance.OpenedChests` (`self.OpenedChests`) GameInstance)
  (set `/Game/ChronoEngine/Blueprints/System/ChronoGameInstance.EventScriptFlags` (`self.EventScriptFlags`) GameInstance)
  (set `/Game/ChronoEngine/Blueprints/System/ChronoGameInstance.EventSwitches` (`self.EventSwitches`) GameInstance)
  (set `/Game/ChronoEngine/Blueprints/System/ChronoGameInstance.EventIntegers` (`self.EventIntegers`) GameInstance)
  (set `/Game/ChronoEngine/Blueprints/System/ChronoGameInstance.EventFloats` (`self.EventFloats`) GameInstance)
  (set `/Game/ChronoEngine/Blueprints/System/ChronoGameInstance.EventStrings` (`self.EventStrings`) GameInstance)
  (`/Game/ChronoEngine/Blueprints/System/ChronoGameInstance.WarpToMap` GameInstance (`self.CurrentMap`) (`self.StartingLocation`)))

(fn `SaveGameInstance`
  (params (GameInstance :type "/Game/ChronoEngine/Blueprints/System/ChronoGameInstance Object Reference") (PlayerLocation :type "Vector Structure"))
  (bind _save (`/Game/ChronoEngine/Blueprints/GameObjects/Party.SaveParty` (`/Game/ChronoEngine/Blueprints/System/ChronoGameInstance.GetParty` GameInstance)))
  (set `self.Party` _save)
  (bind _values (`BlueprintMapLibrary.Map_Values` (`/Game/ChronoEngine/Blueprints/System/ChronoGameInstance.Heroes` GameInstance)))
  (for _array_element _values
    (bind _save_2 (`/Game/ChronoEngine/Blueprints/GameObjects/Hero.SaveHero` _array_element))
    (`BlueprintMapLibrary.Map_Add` (`self.Heros`) (`/Game/ChronoEngine/Blueprints/GameObjects/Hero.GetHeroData` _array_element) _save_2))
  (set `self.CurrentMap` (`/Game/ChronoEngine/Blueprints/System/ChronoGameInstance.CurrentMap` GameInstance))
  (set `self.StartingLocation` (`local.PlayerLocation`))
  (set `self.VisitedMaps` (`/Game/ChronoEngine/Blueprints/System/ChronoGameInstance.VisitedMaps` GameInstance))
  (set `self.OpenedChests` (`/Game/ChronoEngine/Blueprints/System/ChronoGameInstance.OpenedChests` GameInstance))
  (set `self.EventScriptFlags` (`/Game/ChronoEngine/Blueprints/System/ChronoGameInstance.EventScriptFlags` GameInstance))
  (set `self.EventSwitches` (`/Game/ChronoEngine/Blueprints/System/ChronoGameInstance.EventSwitches` GameInstance))
  (set `self.EventIntegers` (`/Game/ChronoEngine/Blueprints/System/ChronoGameInstance.EventIntegers` GameInstance))
  (set `self.EventFloats` (`/Game/ChronoEngine/Blueprints/System/ChronoGameInstance.EventFloats` GameInstance))
  (set `self.EventStrings` (`/Game/ChronoEngine/Blueprints/System/ChronoGameInstance.EventStrings` GameInstance)))