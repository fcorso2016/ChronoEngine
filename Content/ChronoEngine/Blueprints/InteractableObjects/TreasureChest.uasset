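; Treasure chest interactable that opens once when its event script is triggered and stays open through state kept in the ChronoGameInstance.
; Opening swaps the Paper2D flipbook to the open one and records the chest by object name, which BeginPlay checks to restore the open state.
; The OnOpen dispatcher fires only on a triggered open, not on restore.
; The construction script fits the box's X and Y extents to Size.
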(event `self.ReceiveBeginPlay`
  (bind _aschrono_game_instance (cast `/Game/ChronoEngine/Blueprints/System/ChronoGameInstance` (`GameplayStatics.GetGameInstance`)))
  (if (`/Game/ChronoEngine/Blueprints/System/ChronoGameInstance.GetChestOpened?` _aschrono_game_instance (`KismetStringLibrary.Conv_StringToName` (`KismetSystemLibrary.GetObjectName` self)))
    (`self.Open`)))

(event `self.TriggerEventScript`
  (if (not (`self.Opened`))
    (`self.Open`)
    (`self.OnOpen`)))

(fn `Open`
  (set `self.Opened` true)
  (`PaperFlipbookComponent.SetFlipbook` (`self.PaperFlipbook`) "/Game/ChronoEngine/Graphics/Sprites/Objects/ChestOpen_Flipbook.ChestOpen_Flipbook")
  (bind _aschrono_game_instance (cast `/Game/ChronoEngine/Blueprints/System/ChronoGameInstance` (`GameplayStatics.GetGameInstance`)))
  (`/Game/ChronoEngine/Blueprints/System/ChronoGameInstance.OpenChest` _aschrono_game_instance (`KismetStringLibrary.Conv_StringToName` (`KismetSystemLibrary.GetObjectName` self))))

(fn `UserConstructionScript`
  (bind _box (`self.Box`))
  (bind (_x _y) (`KismetMathLibrary.BreakVector2D` (/ (`self.Size`) 2.0)))
  (`BoxComponent.SetBoxExtent` _box (`KismetMathLibrary.MakeVector` _x _y (.z (`BoxComponent.BoxExtent` _box))) true))