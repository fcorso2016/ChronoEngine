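; Action is an RPG data container whose pure-looking query functions classify whom an action can target, based on its TargetType enum.
; Each query compares TargetType to groups of values to report single or multiple targets, ally, enemy or anyone, and whether the user is hit or can be.
; Selection is required for single-target types other than the user-only one, and random targeting applies only when RandomTarget is set on those types.
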(fn `CanHitUser?`
  (returns (ReturnValue :type Boolean))
  (bind _targettype (`self.TargetType`))
  (return (`KismetMathLibrary.BooleanNOR` (`|EnumEquality` _targettype "NewEnumerator9") (`|EnumEquality` _targettype "NewEnumerator7"))))

(fn `HitsAlly?`
  (returns (ReturnValue :type Boolean))
  (bind _targettype (`self.TargetType`))
  (return (or (`|EnumEquality` _targettype "NewEnumerator2") (`|EnumEquality` _targettype "NewEnumerator3") (`|EnumEquality` _targettype "NewEnumerator4"))))

(fn `HitsAnyone?`
  (returns (ReturnValue :type Boolean))
  (bind _targettype (`self.TargetType`))
  (return (or (`|EnumEquality` _targettype "NewEnumerator10") (`|EnumEquality` _targettype "NewEnumerator6") (`|EnumEquality` _targettype "NewEnumerator9") (`|EnumEquality` _targettype "NewEnumerator7"))))

(fn `HitsEnemy?`
  (returns (ReturnValue :type Boolean))
  (bind _targettype (`self.TargetType`))
  (return (or (`|EnumEquality` _targettype "NewEnumerator0") (`|EnumEquality` _targettype "NewEnumerator1"))))

(fn `HitsMultipleTargets?`
  (returns (ReturnValue :type Boolean))
  (bind _targettype (`self.TargetType`))
  (return (or (`|EnumEquality` _targettype "NewEnumerator1") (`|EnumEquality` _targettype "NewEnumerator3") (`|EnumEquality` _targettype "NewEnumerator6") (`|EnumEquality` _targettype "NewEnumerator7"))))

(fn `HitsRandomTarget?`
  (returns (ReturnValue :type Boolean))
  (return (and (`self.RandomTarget?`) (`self.RequiresSelection?`))))

(fn `HitsSingleTarget?`
  (returns (ReturnValue :type Boolean))
  (bind _targettype (`self.TargetType`))
  (return (or (`|EnumEquality` _targettype "NewEnumerator0") (`|EnumEquality` _targettype "NewEnumerator2") (`|EnumEquality` _targettype "NewEnumerator4") (`|EnumEquality` _targettype "NewEnumerator10") (`|EnumEquality` _targettype "NewEnumerator9"))))

(fn `HitsUser?`
  (returns (ReturnValue :type Boolean))
  (return (`|EnumEquality` (`self.TargetType`) "NewEnumerator4")))

(fn `RequiresSelection?`
  (returns (ReturnValue :type Boolean))
  (return (and (`|EnumInequality` (`self.TargetType`) "NewEnumerator4") (`self.HitsSingleTarget?`))))