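; Base battle actor that runs the turn-based combat flow of an RPG, from HUD setup to win/loss judgement.
; Each unit selects an action through a callback, which executes and displays its results.
; After each action, it counts sides able to fight and routes to next action, victory or draw.
; HUD creation, context retrieval, turn-end, result display and outcome handling are empty stubs, apparently for child classes to override.
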(event `BeginActionSelection`
  (params (Unit :type "/Game/RPGBasics/Blueprints/GameObjects/Unit Object Reference"))
  (`/Game/RPGBasics/Blueprints/GameObjects/Unit.SelectAction` Unit (delegate `ExecuteAction`) self))

(event `ExecuteAction`
  (params (Selection :type "Object Object Reference"))
  (bind _asbattle_action (cast `/Game/RPGBasics/Blueprints/Combat/BattleAction` Selection))
  (bind _results (`/Game/RPGBasics/Blueprints/Combat/BattleAction.ExecuteAction` _asbattle_action))
  (for _array_element _results
    (`self.DisplayResult` _array_element))
  (`self.OnActionEnd`))

(fn `BattleEnd`
  (`self.K2_DestroyActor`))

(fn `BattleStart`
  (`self.RetrieveContextInformation`)
  (bind _hud (`self.CreateHUD`))
  (bind _output_get (set `self.HUD` _hud))
  (`/Engine/EditorBlueprintResources/StandardMacros.IsValid` _output_get
    (:`Is Valid`
      (`UserWidget.AddToViewport` _output_get 0))
    (:`Is Not Valid`
      _))
  (bind _returnvalue (`Widget.GetOwningPlayer` _output_get))
  (`WidgetBlueprintLibrary.SetInputMode_UIOnlyEx` _returnvalue _output_get)
  (set `PlayerController.bShowMouseCursor` true _returnvalue)
  (`self.StartTurn`))

(fn `CreateHUD`
  (returns (HUD :type "UserWidget Object Reference"))
  (return null))

(fn `DisplayResult`
  (params (Result :type "/Game/RPGBasics/Blueprints/Combat/ActionResult Object Reference")))

(fn `EndTurn`
  (`self.OnTurnEnd`)
  (`self.StartTurn`))

(fn `GetAllParticipants`
  (returns (Participants :type "Array of /Game/RPGBasics/Blueprints/GameObjects/Unit Object Reference"))
  (locals (Units :type "Array of /Game/RPGBasics/Blueprints/GameObjects/Unit Object Reference"))
  (for _array_element (`self.Sides`)
    (`KismetArrayLibrary.Array_Append` (`local.Units`) (`/Game/RPGBasics/Blueprints/GameObjects/Side.GetMembers` _array_element)))
  (return (`local.Units`)))

(fn `JudgeWinLoss`
  (returns (Result :type "/Game/RPGBasics/Blueprints/Combat/BattleResult Enum") (Winner :type "/Game/RPGBasics/Blueprints/GameObjects/Side Object Reference"))
  (locals (ActiveSides :type "Array of /Game/RPGBasics/Blueprints/GameObjects/Side Object Reference"))
  (bind _activesides (`local.ActiveSides`))
  (for _array_element (`self.Sides`)
    (if (`/Game/RPGBasics/Blueprints/GameObjects/Side.CanFight?` _array_element)
      (`KismetArrayLibrary.Array_Add` (`local.ActiveSides`) _array_element)))
  (switch `int` (`KismetArrayLibrary.Array_Length` _activesides)
    (:`Default`
      (return "NewEnumerator0" null))
    (:`0`
      (return "NewEnumerator2" null))
    (:`1`
      (return "NewEnumerator1" (`|GetArrayItem` _activesides)))))

(fn `NextAction`)

(fn `OnActionEnd`
  (bind (_result _winner) (`self.JudgeWinLoss`))
  (switch `/Game/RPGBasics/Blueprints/Combat/BattleResult` _result
    (:`NewEnumerator0`
      (`self.NextAction`))
    (:`NewEnumerator1`
      (`self.ProcessSideVictory` _winner))
    (:`NewEnumerator2`
      (`self.ProcessDraw`))))

(fn `OnTurnEnd`)

(fn `ProcessDraw`)

(fn `ProcessSideVictory`
  (params (Winner :type "/Game/RPGBasics/Blueprints/GameObjects/Side Object Reference")))

(fn `RetrieveContextInformation`)

(fn `StartTurn`
  (`/Engine/EditorBlueprintResources/StandardMacros.IncrementInt` (`self.TurnCount`)))

(fn `UserConstructionScript`)