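; Battle action object that binds a user, battle context and action data to resolve one RPG combat move.
; SelectTargets fills the target list by custom algorithm, random pick, user, all or single, with pools filtered by side and dead state.
; ExecuteAction runs global effects, then per-target hit, critical, damage and individual effects, returning result objects.
; Targeting and formula modules are constructed from action-specified classes, falling back to defaults; ValidateTargets only prints debug text.
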(fn `ActionTargetsDeadUnits?`
  (returns (`DeadTargets?` :type Boolean))
  (bind _action (`self.Action`))
  (return (select `bool` (`KismetSystemLibrary.IsValid` _action) :`true` (`/Game/RPGBasics/Blueprints/DataContainers/Action.DeadTarget?` _action))))

(fn `CalculateDamage`
  (params (Target :type "/Game/RPGBasics/Blueprints/GameObjects/Unit Object Reference") (`Critical?` :type Boolean))
  (returns (Damage :type Integer))
  (return (`self.ApplyDamageSwing` (`/Game/RPGBasics/Blueprints/Combat/Modules/BaseClasses/FormulaModule.Evaluate` (`self.GetFormulaModule`) (`self.User`) Target `Critical?`))))

(fn `CreateResult`
  (params (ActionType :type "/Game/RPGBasics/Blueprints/Combat/ActionResult Class Reference") (Target :type "/Game/RPGBasics/Blueprints/GameObjects/Unit Object Reference"))
  (returns (Result :type "/Game/RPGBasics/Blueprints/Combat/ActionResult Object Reference"))
  (locals (Res :type "/Game/RPGBasics/Blueprints/Combat/ActionResult Object Reference"))
  (bind _returnvalue (`|GenericCreateObject` ActionType self))
  (bind _output_get (set `local.Res` _returnvalue))
  (`/Game/RPGBasics/Blueprints/Combat/ActionResult.Setup` _output_get Target)
  (return _output_get))

(fn `CustomTargetingAlgorithm`
  (params (Index :type Integer) (Allies :type "Array of /Game/RPGBasics/Blueprints/GameObjects/Unit Object Reference (by ref)") (Enemies :type "Array of /Game/RPGBasics/Blueprints/GameObjects/Unit Object Reference"))
  (returns (Targets :type "Array of /Game/RPGBasics/Blueprints/GameObjects/Unit Object Reference"))
  (return (`/Game/RPGBasics/Blueprints/Combat/Modules/BaseClasses/TargetingModule.Select` (`self.GetTargetingModule`) Index Allies Enemies)))

(fn `DetermineCritical`
  (params (Target :type "/Game/RPGBasics/Blueprints/GameObjects/Unit Object Reference"))
  (returns (`Critical?` :type Boolean))
  (return (`/Game/RPGBasics/Blueprints/Combat/Modules/BaseClasses/CriticalModule.Evaluate` (`self.GetCriticalModule`) 0 (`self.User`) Target)))

(fn `DetermineHit`
  (params (Target :type "/Game/RPGBasics/Blueprints/GameObjects/Unit Object Reference"))
  (returns (`Hit?` :type Boolean))
  (return (`/Game/RPGBasics/Blueprints/Combat/Modules/BaseClasses/HitModule.Evaluate` (`self.GetHitModule`) 0 (`self.User`) Target)))

(fn `EvaluateAction`
  (params (Target :type "/Game/RPGBasics/Blueprints/GameObjects/Unit Object Reference"))
  (returns (TargetResult :type "/Game/RPGBasics/Blueprints/Combat/ActionResult Object Reference") (UserResult :type "/Game/RPGBasics/Blueprints/Combat/ActionResult Object Reference"))
  (locals (TempResult :type "/Game/RPGBasics/Blueprints/Combat/ActionResult Object Reference") (TempResult2 :type "/Game/RPGBasics/Blueprints/Combat/ActionResult Object Reference"))
  (bind _tempresult (`local.TempResult`))
  (bind _result (`self.MakeResult` Target))
  (set `local.TempResult` _result)
  (bind _result_2 (`self.MakeResult` (`self.User`)))
  (set `local.TempResult2` _result_2)
  (if (`self.DetermineHit` Target)
    (`self.EvaluateDamage` (`local.Target`) (`self.CalculateDamage` (`local.Target`) (`self.DetermineCritical` Target)) _tempresult)
    (for _array_element (`/Game/RPGBasics/Blueprints/DataContainers/Action.IndividualEffects` (`self.Action`))
      (bind (_constructedobject _effectchance) (`self.ConstructIndividualEffectEffect` _array_element))
      (`/Game/RPGBasics/Blueprints/Combat/Modules/BaseClasses/IndividualEffectModule.Execute` _constructedobject _effectchance (`self.User`) (`local.Target`) _tempresult)))
  (return _tempresult (`local.TempResult2`)))

(fn `EvaluateDamage`
  (params (Target :type "/Game/RPGBasics/Blueprints/GameObjects/Unit Object Reference") (Damage :type Integer) (Result :type "/Game/RPGBasics/Blueprints/Combat/ActionResult Object Reference"))
  (`/Game/RPGBasics/Blueprints/Combat/Modules/BaseClasses/DamageModule.Apply` (`self.GetDamageModule`) (`self.User`) Target Damage Result null))

(fn `ExecuteAction`
  (returns (Results :type "Array of /Game/RPGBasics/Blueprints/Combat/ActionResult Object Reference"))
  (locals (ResultArray :type "Array of /Game/RPGBasics/Blueprints/Combat/ActionResult Object Reference") (GlobalResult :type "/Game/RPGBasics/Blueprints/Combat/ActionResult Object Reference"))
  (bind _action (`self.Action`))
  (bind _resultarray (`local.ResultArray`))
  (`/Engine/EditorBlueprintResources/StandardMacros.IsValid` _action
    (:`Is Valid`
      (bind _result (`self.CreateResult` (`/Game/RPGBasics/Blueprints/Combat/Battle.ResultClass` (`self.BattleContext`))))
      (bind _output_get (set `local.GlobalResult` _result))
      (`KismetArrayLibrary.Array_Add` (`local.ResultArray`) _output_get)
      (for _array_element (`/Game/RPGBasics/Blueprints/DataContainers/Action.GlobalEffects` _action)
        (bind (_constructedobject _effectchance) (`self.ConstructGlobalEffect` _array_element))
        (`/Game/RPGBasics/Blueprints/Combat/Modules/BaseClasses/GlobalEffectModule.Execute` _constructedobject _effectchance (`self.User`) (`local.GlobalResult`)))
      (for _array_element_2 (`self.Targets`)
        (bind (_targetresult _userresult) (`self.EvaluateAction` _array_element_2))
        (`KismetArrayLibrary.Array_Add` _resultarray _targetresult)
        (`KismetArrayLibrary.Array_Add` _resultarray _userresult))
      (return (`local.ResultArray`)))))

(fn `GetAction`
  (returns (Action :type "/Game/RPGBasics/Blueprints/DataContainers/Action Object Reference"))
  (return (`self.Action`)))

(fn `GetAllAllies`
  (returns (Allies :type "Array of /Game/RPGBasics/Blueprints/GameObjects/Unit Object Reference"))
  (return (`/Game/RPGBasics/Blueprints/GameObjects/Side.GetMembers` (`/Game/RPGBasics/Blueprints/GameObjects/Unit.GetSide` (`self.User`)))))

(fn `GetAllEnemies`
  (returns (Enemies :type "Array of /Game/RPGBasics/Blueprints/GameObjects/Unit Object Reference"))
  (locals (TempSides :type "Array of /Game/RPGBasics/Blueprints/GameObjects/Side Object Reference") (EnemyList :type "Array of /Game/RPGBasics/Blueprints/GameObjects/Unit Object Reference"))
  (bind _output_get (set `local.TempSides` (`/Game/RPGBasics/Blueprints/Combat/Battle.Sides` (`self.BattleContext`))))
  (`KismetArrayLibrary.Array_RemoveItem` _output_get (`/Game/RPGBasics/Blueprints/GameObjects/Unit.GetSide` (`self.User`)))
  (for _array_element _output_get
    (`KismetArrayLibrary.Array_Append` (`local.EnemyList`) (`/Game/RPGBasics/Blueprints/GameObjects/Side.GetMembers` _array_element)))
  (return (`local.EnemyList`)))

(fn `GetAllPossibleTargets`
  (returns (Targets :type "Array of /Game/RPGBasics/Blueprints/GameObjects/Unit Object Reference"))
  (locals (TempTargets :type "Array of /Game/RPGBasics/Blueprints/GameObjects/Unit Object Reference"))
  (bind _output_get (set `local.TempTargets` (`self.GetAllAllies`)))
  (`KismetArrayLibrary.Array_Append` _output_get (`self.GetAllEnemies`))
  (return (`local.TempTargets`)))

(fn `GetCriticalModule`
  (returns (Module :type "/Game/RPGBasics/Blueprints/Combat/Modules/BaseClasses/CriticalModule Object Reference"))
  (bind _returnvalue (`|GenericCreateObject` (`/Game/RPGBasics/Blueprints/DataContainers/Action.CriticalFormula` (`self.Action`)) self))
  (`/Engine/EditorBlueprintResources/StandardMacros.IsValid` _returnvalue
    (:`Is Valid`
      (return _returnvalue))
    (:`Is Not Valid`
      (bind _returnvalue_2 (`|GenericCreateObject` "/Game/RPGBasics/Blueprints/Combat/Modules/BaseClasses/CriticalModule.CriticalModule_C" self))
      (return _returnvalue_2))))

(fn `GetDamageModule`
  (returns (Module :type "/Game/RPGBasics/Blueprints/Combat/Modules/BaseClasses/DamageModule Object Reference"))
  (bind _returnvalue (`|GenericCreateObject` (`/Game/RPGBasics/Blueprints/DataContainers/Action.DamageType` (`self.Action`)) self))
  (`/Engine/EditorBlueprintResources/StandardMacros.IsValid` _returnvalue
    (:`Is Valid`
      (return _returnvalue))
    (:`Is Not Valid`
      (bind _returnvalue_2 (`|GenericCreateObject` "/Game/RPGBasics/Blueprints/Combat/Modules/BaseClasses/DamageModule.DamageModule_C" self))
      (return _returnvalue_2))))

(fn `GetFormulaModule`
  (returns (Module :type "/Game/RPGBasics/Blueprints/Combat/Modules/BaseClasses/FormulaModule Object Reference"))
  (bind _returnvalue (`|GenericCreateObject` (`/Game/RPGBasics/Blueprints/DataContainers/Action.DamageFormula` (`self.Action`)) self))
  (`/Engine/EditorBlueprintResources/StandardMacros.IsValid` _returnvalue
    (:`Is Valid`
      (return _returnvalue))
    (:`Is Not Valid`
      (bind _returnvalue_2 (`|GenericCreateObject` "/Game/RPGBasics/Blueprints/Combat/Modules/BaseClasses/FormulaModule.FormulaModule_C" self))
      (return _returnvalue_2))))

(fn `GetHitModule`
  (returns (Module :type "/Game/RPGBasics/Blueprints/Combat/Modules/BaseClasses/HitModule Object Reference"))
  (bind _returnvalue (`|GenericCreateObject` (`/Game/RPGBasics/Blueprints/DataContainers/Action.HitFormula` (`self.Action`)) self))
  (`/Engine/EditorBlueprintResources/StandardMacros.IsValid` _returnvalue
    (:`Is Valid`
      (return _returnvalue))
    (:`Is Not Valid`
      (bind _returnvalue_2 (`|GenericCreateObject` "/Game/RPGBasics/Blueprints/Combat/Modules/BaseClasses/HitModule.HitModule_C" self))
      (return _returnvalue_2))))

(fn `GetRandomTarget`
  (params (TargetChoices :type "Array of /Game/RPGBasics/Blueprints/GameObjects/Unit Object Reference"))
  (returns (Target :type "/Game/RPGBasics/Blueprints/GameObjects/Unit Object Reference"))
  (return (`|GetArrayItem` TargetChoices (`KismetMathLibrary.RandomInteger` (- (`KismetArrayLibrary.Array_Length` TargetChoices) 1)))))

(fn `GetTargetingModule`
  (returns (Module :type "/Game/RPGBasics/Blueprints/Combat/Modules/BaseClasses/TargetingModule Object Reference"))
  (bind _returnvalue (`|GenericCreateObject` (`/Game/RPGBasics/Blueprints/DataContainers/Action.CustomTargetingAlgorithm` (`self.Action`)) self))
  (`/Engine/EditorBlueprintResources/StandardMacros.IsValid` _returnvalue
    (:`Is Valid`
      (return _returnvalue))
    (:`Is Not Valid`
      (bind _returnvalue_2 (`|GenericCreateObject` "/Game/RPGBasics/Blueprints/Combat/Modules/BaseClasses/TargetingModule.TargetingModule_C" self))
      (return _returnvalue_2))))

(fn `GetTargetPool`
  (returns (Targets :type "Array of /Game/RPGBasics/Blueprints/GameObjects/Unit Object Reference"))
  (locals (ReturnTargets :type "Array of /Game/RPGBasics/Blueprints/GameObjects/Unit Object Reference") (Index :type Integer))
  (bind _action (`self.Action`))
  (bind _returntargets (`local.ReturnTargets`))
  (bind _index (`local.Index`))
  (`/Engine/EditorBlueprintResources/StandardMacros.IsValid` (`self.Action`)
    (:`Is Valid`
      (`self.DoubleBranch` (`/Game/RPGBasics/Blueprints/DataContainers/Action.HitsAlly?` _action) (`/Game/RPGBasics/Blueprints/DataContainers/Action.HitsEnemy?` _action)
        (:`IfCondition1`
          (set `local.ReturnTargets` (`self.GetAllAllies`)))
        (:`IfCondition2`
          (set `local.ReturnTargets` (`self.GetAllEnemies`)))
        (:`Else`
          (set `local.ReturnTargets` (`self.GetAllPossibleTargets`))))
      (if (not (`/Game/RPGBasics/Blueprints/DataContainers/Action.CanHitUser?` (`self.Action`)))
        (`KismetArrayLibrary.Array_RemoveItem` _returntargets (`self.User`)))
      (while (< (`local.Index`) (`KismetArrayLibrary.Array_Length` _returntargets))
        (if (!= (`/Game/RPGBasics/Blueprints/GameObjects/Unit.IsDead?` (`|GetArrayItem` _returntargets (`local.Index`))) (`self.ActionTargetsDeadUnits?`))
          (`KismetArrayLibrary.Array_Remove` _returntargets _index)
          (else
            (`/Engine/EditorBlueprintResources/StandardMacros.IncrementInt` _index))))
      (return _returntargets))
    (:`Is Not Valid`
      (return (`local.ReturnTargets`)))))

(fn `GetTargetType`
  (returns (TargetType :type "/Game/RPGBasics/Blueprints/GameObjects/TargetType Enum"))
  (bind _action (`self.Action`))
  (return (select `bool` (`KismetSystemLibrary.IsValid` _action) :`false` "NewEnumerator5" :`true` (`/Game/RPGBasics/Blueprints/DataContainers/Action.TargetType` _action))))

(fn `SelectAllTargets`
  (`self.DoX_Times` (`self.RandomIntInRange` (`/Game/RPGBasics/Blueprints/DataContainers/Action.NumberOfHits` (`self.Action`)))
    (:`LoopBody`
      (`KismetArrayLibrary.Array_Append` (`self.Targets`) (`self.GetTargetPool`)))))

(fn `SelectRandomTarget`
  (locals (RandomTarget :type "/Game/RPGBasics/Blueprints/GameObjects/Unit Object Reference"))
  (bind _action (`self.Action`))
  (bind _target (`self.GetRandomTarget` (`self.GetTargetPool`)))
  (bind _selectedint (`self.RandomIntInRange` (`/Game/RPGBasics/Blueprints/DataContainers/Action.NumberOfHits` _action)))
  (if (`/Game/RPGBasics/Blueprints/DataContainers/Action.HitRetarget` _action)
    (`self.DoX_Times` _selectedint
      (:`LoopBody`
        (`KismetArrayLibrary.Array_Add` (`self.Targets`) _target)))
    (else
      (bind _output_get (set `local.RandomTarget` _target))
      (`self.DoX_Times` _selectedint
        (:`LoopBody`
          (`KismetArrayLibrary.Array_Add` (`self.Targets`) _output_get))))))

(fn `SelectSingleTarget`
  (params (Index :type Integer))
  (`self.DoX_Times` (`self.RandomIntInRange` (`/Game/RPGBasics/Blueprints/DataContainers/Action.NumberOfHits` (`self.Action`)))
    (:`LoopBody`
      (set `self.Targets` (`|MakeArray` (`|GetArrayItem` (`self.GetTargetPool`) Index))))))

(fn `SelectTargets`
  (params (TargetIndex :type Integer))
  (locals (RandomTarget :type "/Game/RPGBasics/Blueprints/GameObjects/Unit Object Reference"))
  (bind _action (`self.Action`))
  (bind _action_2 (`self.Action`))
  (`/Engine/EditorBlueprintResources/StandardMacros.IsValid` _action
    (:`Is Valid`
      (if (`|EnumEquality` (`/Game/RPGBasics/Blueprints/DataContainers/Action.TargetType` _action) "NewEnumerator8")
        (set `self.Targets` (`self.CustomTargetingAlgorithm` TargetIndex (`self.GetAllAllies`) (`self.GetAllEnemies`)))
        (elif (`/Game/RPGBasics/Blueprints/DataContainers/Action.HitsRandomTarget?` _action_2)
          (`self.SelectRandomTarget`)
          (elif (`/Game/RPGBasics/Blueprints/DataContainers/Action.HitsUser?` _action_2)
            (`self.SelectUser`)
            (elif (`/Game/RPGBasics/Blueprints/DataContainers/Action.HitsMultipleTargets?` _action_2)
              (`self.SelectAllTargets`)
              (else
                (`self.SelectSingleTarget` TargetIndex)))))))))

(fn `SelectUser`
  (`self.DoX_Times` (`self.RandomIntInRange` (`/Game/RPGBasics/Blueprints/DataContainers/Action.NumberOfHits` (`self.Action`)))
    (:`LoopBody`
      (`KismetArrayLibrary.Array_Add` (`self.Targets`) (`self.User`)))))

(fn `SetAction`
  (params (Action :type "/Game/RPGBasics/Blueprints/DataContainers/Action Object Reference"))
  (set `self.Action` Action))

(fn `Setup`
  (params (Battle :type "/Game/RPGBasics/Blueprints/Combat/Battle Object Reference") (User :type "/Game/RPGBasics/Blueprints/GameObjects/Unit Object Reference") (Action :type "/Game/RPGBasics/Blueprints/DataContainers/Action Object Reference"))
  (set `self.BattleContext` Battle)
  (set `self.User` User)
  (set `self.Action` Action))

(fn `ValidateTargets`
  (params (targets :type "Array of /Game/RPGBasics/Blueprints/GameObjects/Unit Object Reference"))
  (for _array_element targets
    (if (`/Game/RPGBasics/Blueprints/GameObjects/Unit.IsDead?` _array_element)
      (`KismetSystemLibrary.PrintText` (`self.BattleContext`) "Hello"))))