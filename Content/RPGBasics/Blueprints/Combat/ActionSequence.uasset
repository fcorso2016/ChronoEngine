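; ActionSequence is a base actor that sequences one battle action in the RPG combat system, from ready pose to completion.
; UseAction processes the cost and starts activation; completion callbacks then advance through animation, effect execution, results display and post-action steps.
; Presentation and cost steps are empty hooks, apparently meant for child overrides.
; When finished, it destroys itself and notifies the owning battle through OnActionEnd.
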(fn `ApplyActionEffects`
  (bind _results (`/Game/RPGBasics/Blueprints/Combat/BattleAction.ExecuteAction` (`self.Action`)))
  (`self.DisplayActionResults` _results))

(fn `CallActionAnimation`)

(fn `CallActivationSequence`)

(fn `CallPostActionSequence`)

(fn `DisplayActionResults`
  (params (Results :type "Array of /Game/RPGBasics/Blueprints/Combat/ActionResult Object Reference (by ref)")))

(fn `OnActivationComplete`
  (`self.CallActionAnimation`))

(fn `OnAnimationComplete`
  (`self.ApplyActionEffects`))

(fn `OnResultsDisplayComplete`
  (`self.CallPostActionSequence`)
  (`self.Terminate`))

(fn `ProcessActionCost`)

(fn `ProcessWinLossJudgement`
  (params (Selection :type "/Game/RPGBasics/Blueprints/Combat/BattleResult Enum" :default "NewEnumerator0") (InputPin :type "/Game/RPGBasics/Blueprints/GameObjects/Side Object Reference"))
  (switch `/Game/RPGBasics/Blueprints/Combat/BattleResult` Selection))

(fn `ReadyPose`)

(fn `SetupAction`
  (params (Action :type "/Game/RPGBasics/Blueprints/Combat/BattleAction Object Reference") (OwningBattle :type "/Game/RPGBasics/Blueprints/Combat/Battle Object Reference"))
  (set `self.Action` Action)
  (set `self.OwningBattle` OwningBattle)
  (`self.ReadyPose`))

(fn `Terminate`
  (`self.K2_DestroyActor`)
  (`/Game/RPGBasics/Blueprints/Combat/Battle.OnActionEnd` (`self.OwningBattle`)))

(fn `UseAction`
  (set `self.Running` true)
  (`self.ProcessActionCost`)
  (`self.CallActivationSequence`))

(fn `UserConstructionScript`)