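; Unit is a base Blueprint for an RPG combat unit that tracks HP, owning side and death state.
; HP changes from damage or healing pass through SetCurrentHP, which clamps to max HP and calls Die at zero.
; Battle speed, max HP and damage rate per attack type return placeholder values, apparently for child classes to override.
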(fn `Die`
  (set `self.HP` 0))

(fn `GetBattleSpeed`
  (returns (Speed :type Integer))
  (return 0))

(fn `GetCurrentHP`
  (returns (HP :type Integer))
  (return (`self.HP`)))

(fn `GetDamageRate`
  (params (AttckType :type "/Game/RPGBasics/Blueprints/Combat/Modules/BaseClasses/AttackType Enum" :default "NewEnumerator0"))
  (returns (DamageRate :type "Float (double-precision)"))
  (return 1.0))

(fn `GetMaxHP`
  (returns (HP :type Integer))
  (return 0))

(fn `GetSide`
  (returns (Side :type "/Game/RPGBasics/Blueprints/GameObjects/Side Object Reference"))
  (return (`self.OwningSide`)))

(fn `IsDead?`
  (returns (`Dead?` :type Boolean))
  (return (== (`self.HP`) 0)))

(fn `SetCurrentHP`
  (params (NewHP :type Integer))
  (bind _output_get (set `self.HP` (`KismetMathLibrary.Clamp` NewHP 0 (`self.GetMaxHP`))))
  (if (== _output_get 0)
    (`self.Die`)))

(fn `TakeDamage/Heal`
  (params (Amount :type Integer) (ChangeType :type "/Game/RPGBasics/Blueprints/GameObjects/ChangeType Enum" :default "NewEnumerator0"))
  (switch `/Game/RPGBasics/Blueprints/GameObjects/ChangeType` ChangeType
    (:`NewEnumerator0`
      (`self.SetCurrentHP` (+ (`self.HP`) Amount)))
    (:`NewEnumerator1`
      (`self.SetCurrentHP` (- (`self.HP`) Amount)))))