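; Side Blueprint that represents a group of combatants in the RPG basics and reports whether that group can still fight.
; GetMembers returns an empty list here, serving as a placeholder for the group's roster.
; CanFight? loops over that roster, folds each member's IsDead result into an AllDead flag with AND, and returns the negation.
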(fn `CanFight?`
  (returns (ReturnValue :type Boolean))
  (locals (`AllDead?` :type Boolean :default true))
  (for _array_element (`self.GetMembers`)
    (set `local.AllDead?` (and (`/Game/RPGBasics/Blueprints/GameObjects/Unit.IsDead?` _array_element) (`local.AllDead?`))))
  (return (not (`local.AllDead?`))))

(fn `GetMembers`
  (returns (Members :type "Array of /Game/RPGBasics/Blueprints/GameObjects/Unit Object Reference"))
  (return (`|MakeArray`)))