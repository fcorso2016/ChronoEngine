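; ATB_Battle is a battle Blueprint that extends a parent battle class with party notification and HUD creation.
; On BattleStart it casts the game instance to ChronoGameInstance and tells its party the battle has started, then runs the parent logic, which is skipped if the cast fails.
; CreateHUD builds a BattleHUD widget for player controller 0, calls its Setup and returns it.
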(event `self.BattleStart`
  (bind _aschrono_game_instance (cast `/Game/Blueprints/System/ChronoGameInstance` (`GameplayStatics.GetGameInstance`)))
  (`/Game/Blueprints/GameObjects/Party.OnStartBattle` (`/Game/Blueprints/System/ChronoGameInstance.GetParty` _aschrono_game_instance))
  (`parent.BattleStart`))

(fn `CreateHUD`
  (returns (HUD :type "UserWidget Object Reference"))
  (bind _returnvalue (`|CreateWidget` "/Game/UI/Combat/Menus/BattleHUD.BattleHUD_C" (`GameplayStatics.GetPlayerController` 0)))
  (`/Game/UI/Combat/Menus/BattleHUD.Setup` _returnvalue)
  (return _returnvalue))

(fn `UserConstructionScript`
  (`parent.UserConstructionScript`))