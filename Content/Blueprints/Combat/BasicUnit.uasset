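; BasicUnit is a battle unit that rolls its own stats and picks its own action without player input.
; Initialize randomizes max HP, attack and defense within fixed ranges and starts HP at the maximum.
; SelectAction rebinds the selection-complete delegate, builds an Attack BattleAction, sets its targets through SelectRandom on the target pool, then fires the delegate immediately.
; The SelectRandom graph holds only an unconnected random-index node.
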(event `self.Initialize`
  (bind _output_get (set `self.MaxHP` (`KismetMathLibrary.RandomIntegerInRange` 20 30)))
  (set `self.HP` _output_get)
  (set `self.Attack` (`KismetMathLibrary.RandomIntegerInRange` 10 15))
  (set `self.Defense` (`KismetMathLibrary.RandomIntegerInRange` 5 10)))

(event `self.SelectAction`
  (params (OnInputComplete :type "Delegate (by ref)") (Object :type "Object Object Reference"))
  (clear `self.OnSelectionComplete`)
  (add `self.OnSelectionComplete` OnInputComplete)
  (bind _returnvalue (`|GenericCreateObject` "/RPGBasics/Blueprints/Combat/BattleAction.BattleAction_C" self))
  (bind _asbattle (cast `/RPGBasics/Blueprints/Combat/Battle` Object))
  (`/RPGBasics/Blueprints/Combat/BattleAction.Setup` _returnvalue _asbattle self "/Game/Data/Skills/Attack.Attack")
  (`/RPGBasics/Blueprints/Combat/BattleAction.SelectTargets` _returnvalue (`self.SelectRandom` (`/RPGBasics/Blueprints/Combat/BattleAction.GetTargetPool` _returnvalue)))
  (`self.OnSelectionComplete` _returnvalue))