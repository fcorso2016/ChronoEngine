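; Turn-based battle Blueprint that orders units by speed and prints turns, damage and the winner or draw as text.
; Each turn sorts all participants via a comparator, apparently CompareSpeed with its DoubleCast macro, then begins action selection for the first.
; NextAction pops that unit and continues, ending the turn when the order empties.
; Battle context is built in code as two sides, each holding one BasicUnit.
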(event `self.StartTurn`
  (`parent.StartTurn`)
  (`KismetSystemLibrary.PrintText` (`|FormatText` "Turn: {Turn No.}" (`self.TurnCount`)))
  (`self.CreateTurnOrder`)
  (`self.ProcessAction`))

(event `self.NextAction`
  (`parent.NextAction`)
  (`KismetArrayLibrary.Array_Remove` (`self.TurnOrder`))
  (`self.ProcessAction`))

(event `self.RetrieveContextInformation`
  (for _ (range 2)
    (bind _returnvalue (`|GenericCreateObject` "/RPGBasics/Blueprints/GameObjects/Side.Side_C" self))
    (bind _returnvalue_2 (`|GenericCreateObject` "/Game/Blueprints/Combat/BasicUnit.BasicUnit_C" self))
    (set `/RPGBasics/Blueprints/GameObjects/Unit.OwningSide` _returnvalue _returnvalue_2)
    (`KismetArrayLibrary.Array_Add` (`/RPGBasics/Blueprints/GameObjects/Side.Members` _returnvalue) _returnvalue_2)
    (`KismetArrayLibrary.Array_Add` (`self.Sides`) _returnvalue)))

(event `self.ProcessSideVictory`
  (params (Winner :type "/RPGBasics/Blueprints/GameObjects/Side Object Reference"))
  (`KismetSystemLibrary.PrintText` (`|FormatText` "Winner: Side {Winner}" (`KismetArrayLibrary.Array_Find` (`self.Sides`) Winner))))

(event `self.ProcessDraw`
  (`KismetSystemLibrary.PrintText` "Draw!"))

(event `self.DisplayResult`
  (params (Result :type "/RPGBasics/Blueprints/Combat/ActionResult Object Reference"))
  (`KismetSystemLibrary.PrintText` (`|FormatText` "{Damage} Damage" (* (`/RPGBasics/Blueprints/Combat/ActionResult.TargetHP_Change` Result) -1))))

(fn `CompareSpeed`
  (params (Unit1 :type "Object Object Reference") (Unit2 :type "Object Object Reference"))
  (returns (Unit1_First :type Boolean))
  (bind (_asunit _asunit2) (`self.DoubleCast` Unit1 Unit2)
    (:`then`
      (return (> (`/RPGBasics/Blueprints/GameObjects/Unit.GetBattleSpeed` _asunit) (`/RPGBasics/Blueprints/GameObjects/Unit.GetBattleSpeed` _asunit2))))
    (:`CastFailed`
      (return false))))

(fn `CreateTurnOrder`
  (bind _output_get (set `self.TurnOrder` (`self.GetAllParticipants`)))
  (`LowEntryExtendedStandardLibrary.SortObjectArrayDirectly` _output_get (`|CreateDelegate` :!event `CompareSpeed`)))

(fn `ProcessAction`
  (bind _turnorder (`self.TurnOrder`))
  (if (> (`KismetArrayLibrary.Array_Length` _turnorder) 0)
    (`self.BeginActionSelection` (`|GetArrayItem` _turnorder))
    (else
      (`self.EndTurn`))))

(fn `UserConstructionScript`
  (`parent.UserConstructionScript`))