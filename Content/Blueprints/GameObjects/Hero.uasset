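; Hero is a battle unit object whose base stats and level cap come from a HeroData asset.
; Setup stores the owning side and data, then fills current HP and MP to maximum.
; GetBaseStat routes stat curves through EvaluateStatCurve, currently a stub returning 0, while Speed is read directly.
; SetLevel clamps to GetMaxLevel, which reads a separate HeroData variable, defaulting to 99 if invalid.
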(fn `EvaluateStatCurve`
  (params (Curve :type "CurveTableRowHandle Structure"))
  (returns (Stat :type Integer))
  (return 0))

(fn `GetBaseStat`
  (params (Stat :type "/Game/Blueprints/GameObjects/Stat Enum" :default "NewEnumerator0"))
  (returns (Value :type Integer))
  (bind _herodata (`self.GetHeroData`))
  (return (select `bool` (`KismetSystemLibrary.IsValid` _herodata) :`true` (select `/Game/Blueprints/GameObjects/Stat` Stat :`NewEnumerator0` (`self.EvaluateStatCurve` (`/Game/Blueprints/DataObjects/HeroData.BaseHP` _herodata)) :`NewEnumerator1` (`self.EvaluateStatCurve` (`/Game/Blueprints/DataObjects/HeroData.BaseMP` _herodata)) :`NewEnumerator2` (`self.EvaluateStatCurve` (`/Game/Blueprints/DataObjects/HeroData.BaseAttack` _herodata)) :`NewEnumerator3` (`self.EvaluateStatCurve` (`/Game/Blueprints/DataObjects/HeroData.BaseDefense` _herodata)) :`NewEnumerator4` (`self.EvaluateStatCurve` (`/Game/Blueprints/DataObjects/HeroData.BaseMagic` _herodata)) :`NewEnumerator5` (`self.EvaluateStatCurve` (`/Game/Blueprints/DataObjects/HeroData.BaseResistance` _herodata)) :`NewEnumerator6` (`/Game/Blueprints/DataObjects/HeroData.BaseSpeed` _herodata)))))

(fn `GetHeroData`
  (returns (HeroData :type "/Game/Blueprints/DataObjects/HeroData Object Reference"))
  (bind _ashero_data (cast `/Game/Blueprints/DataObjects/HeroData` (`self.UnitData`))
    (:`then`
      (return _ashero_data))
    (:`CastFailed`
      (return null))))

(fn `GetLevel`
  (returns (Level :type Integer))
  (return (`self.Level`)))

(fn `GetMaxLevel`
  (returns (MaxLevel :type Integer))
  (bind _herodata (`self.HeroData`))
  (return (select `bool` (`KismetSystemLibrary.IsValid` _herodata) :`false` 99 :`true` (`/Game/Blueprints/DataObjects/HeroData.MaxLevel` _herodata))))

(fn `SetLevel`
  (params (Level :type Integer))
  (set `self.Level` (`KismetMathLibrary.Clamp` Level 1 (`self.GetMaxLevel`))))

(fn `Setup`
  (params (GameInstance :type "GameInstance Object Reference") (OwningSide :type "/RPGBasics/Blueprints/GameObjects/Side Object Reference") (DataObject :type "/Game/Blueprints/DataObjects/HeroData Object Reference"))
  (set `self.OwningSide` OwningSide)
  (set `self.UnitData` DataObject)
  (`self.SetCurrentHP` (`self.GetMaxHP`))
  (`self.SetCurrentMP` (`self.GetMaxMP`)))