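; Combatant is a base for RPG battle participants, exposing HP, MP, attack, defense, magic, resistance, speed, level and hit, evasion and critical chances.
; Named getters route through GetStat, which combines base value, multiplier and bonus from placeholder functions that return neutral defaults, presumably for child overrides.
; GetStat clamps using the first enumerator's (HP) limits, whatever stat is requested.
; Current MP is stored and clamped between zero and max MP.
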(fn `GetAttack`
  (returns (Attack :type Integer))
  (return (`self.GetStat` "NewEnumerator2")))

(fn `GetBaseStat`
  (params (Stat :type "/Game/Blueprints/GameObjects/Stat Enum" :default "NewEnumerator0"))
  (returns (Value :type Integer))
  (return 0))

(fn `GetBattleSpeed`
  (returns (Speed :type Integer))
  (return (`self.GetSpeed`)))

(fn `GetCriticalChance`
  (returns (Critical :type Integer))
  (return 4))

(fn `GetCurrentMP`
  (returns (MP :type Integer))
  (return (`self.MP`)))

(fn `GetDefense`
  (returns (Defense :type Integer))
  (return (`self.GetStat` "NewEnumerator3")))

(fn `GetEvasion`
  (returns (Evasion :type Integer))
  (return 5))

(fn `GetHit`
  (returns (Hit :type Integer))
  (return 95))

(fn `GetLevel`
  (returns (Level :type Integer))
  (return 0))

(fn `GetMagic`
  (returns (Magic :type Integer))
  (return (`self.GetStat` "NewEnumerator4")))

(fn `GetMaxHP`
  (returns (HP :type Integer))
  (return (`self.GetStat` "NewEnumerator0")))

(fn `GetMaxMP`
  (returns (MP :type Integer))
  (return (`self.GetStat` "NewEnumerator1")))

(fn `GetResistance`
  (returns (Resistance :type Integer))
  (return (`self.GetStat` "NewEnumerator5")))

(fn `GetSpeed`
  (returns (Speed :type Integer))
  (return (`self.GetStat` "NewEnumerator6")))

(fn `GetStat`
  (params (Stat :type "/Game/Blueprints/GameObjects/Stat Enum" :default "NewEnumerator0"))
  (returns (Value :type Integer))
  (return (`KismetMathLibrary.Clamp` (`KismetMathLibrary.FTrunc` (+ (* (`self.GetBaseStat` Stat) (`self.GetStatMultipliers` Stat)) (`KismetMathLibrary.Conv_IntToDouble` (`self.GetStatBonus` Stat)))) (`self.GetStatMin` "NewEnumerator0") (`self.GetStatMax` "NewEnumerator0"))))

(fn `GetStatBonus`
  (params (Stat :type "/Game/Blueprints/GameObjects/Stat Enum" :default "NewEnumerator0"))
  (returns (Bonus :type Integer))
  (return 0))

(fn `GetStatMax`
  (params (Stat :type "/Game/Blueprints/GameObjects/Stat Enum" :default "NewEnumerator0"))
  (returns (Max :type Integer))
  (return (select `bool` (`|EnumEquality` Stat "NewEnumerator6") :`false` 999 :`true` 16)))

(fn `GetStatMin`
  (params (Stat :type "/Game/Blueprints/GameObjects/Stat Enum" :default "NewEnumerator0"))
  (returns (Max :type Integer))
  (return (select `bool` (`|EnumEquality` Stat "NewEnumerator1") :`false` 1)))

(fn `GetStatMultipliers`
  (params (Stat :type "/Game/Blueprints/GameObjects/Stat Enum" :default "NewEnumerator0"))
  (returns (Multiplier :type "Float (double-precision)"))
  (return 1.0))

(fn `SetCurrentMP`
  (params (MP :type Integer))
  (set `self.MP` (`KismetMathLibrary.Clamp` MP 0 (`self.GetMaxMP`))))