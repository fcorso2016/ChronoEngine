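; HeroData is a hero data object that checks its starting equipment when property validation runs.
; ValidatePropertyInformation calls ValidateEquipment, which loops over InitialEquips and replaces any slot failing ValidateEquipmentClass with the result of DequipItem.
; The helpers hold nodes for comparing a piece's class to its slot's EquipmentType and rebuilding a slot from its type, both marked unused.
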(event `self.ValidatePropertyInformation`
  (`self.ValidateEquipment`))